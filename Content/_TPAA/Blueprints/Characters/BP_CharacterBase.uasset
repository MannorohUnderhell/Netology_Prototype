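; BP_CharacterBase is a base character Blueprint that lets a character use nearby interactable actors.
; InteractSphere overlaps store any actor implementing BI_Interaction in ActorToInteract, and end overlap with any such actor clears it.
; ActionUse sends InteractMessage to the stored actor if valid, passing the character as the argument.
; Only one target is tracked, so leaving one interactable clears the target even if another still overlaps.
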(event `self.InteractSphere.OnComponentBeginOverlap`
  (params (OverlappedComponent :type "PrimitiveComponent Object Reference") (OtherActor :type "Actor Object Reference") (OtherComp :type "PrimitiveComponent Object Reference") (OtherBodyIndex :type Integer) (bFromSweep :type Boolean) (SweepResult :type "HitResult Structure (by ref)"))
  ; Overlap logic for Actor to Interact
  (if (`KismetSystemLibrary.DoesImplementInterface` OtherActor "/Game/_TPAA/Blueprints/GameEntities/BI_Interaction.BI_Interaction_C")
    (set `self.ActorToInteract` OtherActor)))

(event `self.InteractSphere.OnComponentEndOverlap`
  (params (OverlappedComponent :type "PrimitiveComponent Object Reference") (OtherActor :type "Actor Object Reference") (OtherComp :type "PrimitiveComponent Object Reference") (OtherBodyIndex :type Integer))
  ; Overlap logic for Actor to Interact
  (if (`KismetSystemLibrary.DoesImplementInterface` OtherActor "/Game/_TPAA/Blueprints/GameEntities/BI_Interaction.BI_Interaction_C")
    (set `self.ActorToInteract` null)))

(fn `ActionUse`
  (bind _actortointeract (`self.ActorToInteract`)
    (:`then`
      (message `/Game/_TPAA/Blueprints/GameEntities/BI_Interaction.Interact` _actortointeract self))
    (:`else`)))

(fn `UserConstructionScript`)