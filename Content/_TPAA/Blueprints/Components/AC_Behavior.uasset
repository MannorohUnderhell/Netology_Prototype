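; Actor component that sets up its owner's behavior and faction from the owner's main stats.
; On BeginPlay it requests the main stats struct from the owner through a message call and, on success, caches the current behavior and faction.
; It then fires the OnBehaviorUpdate dispatcher, passing both along with the attack, chase and retreat distances for listeners to use.
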(event `self.ReceiveBeginPlay`
  (`self.ConfigureBehaviorAndFactions`))

(fn `ConfigureBehaviorAndFactions`
  (locals (L_MainStats :type "/Game/_TPAA/Blueprints/Structures/STRUCT_MainStats Structure"))
  (bind ((`Behavior_18_0AA5276749D3D1C45A0A768D3168730B` _behavior) (`Faction_20_0B0BB877412A3F8175648EB4E413CEE7` _faction) (`AttackStartDistance_31_6938B31B41412F94014F39A70B56E561` _attackstartdistance) (`ChaseStartDistance_32_0787EE1C4EB122F884D105929EA072F0` _chasestartdistance) (`RetreatStartDistance_33_4934857041627BFE7C49AB82EA312530` _retreatstartdistance) (`RetreatDistance_34_DFCABB0949AE840D415D0CAFF96C7EAE` _retreatdistance)) (break `/Game/_TPAA/Blueprints/Structures/STRUCT_MainStats` (`local.L_MainStats`)))
  (bind (_success _mainstats) (message `/Game/_TPAA/Blueprints/GameEntities/BI_Stats.GetMainStatsStruct` (`self.GetOwner`)))
  (if _success
    (set `local.L_MainStats` _mainstats)
    (`|ExecutionSequence`
      (:`then_0`
        (`self.UpdateBehavior` (`.Behavior_18_0AA5276749D3D1C45A0A768D3168730B` (break `/Game/_TPAA/Blueprints/Structures/STRUCT_MainStats` (`local.L_MainStats`))))
        (`self.UpdateFaction` (`.Faction_20_0B0BB877412A3F8175648EB4E413CEE7` (break `/Game/_TPAA/Blueprints/Structures/STRUCT_MainStats` (`local.L_MainStats`)))))
      (:`then_1`
        (`self.OnBehaviorUpdate` _behavior _faction _attackstartdistance _chasestartdistance _retreatstartdistance _retreatdistance)))))

(fn `UpdateBehavior`
  (params (InCurrentBehavior :type "/Game/_TPAA/Blueprints/Enums/ENUM_Behavior Enum" :default "NewEnumerator0"))
  (set `self.CurrentBehavior` InCurrentBehavior))

(fn `UpdateFaction`
  (params (CurrentFaction :type "/Game/_TPAA/Blueprints/Enums/ENUM_Faction Enum" :default "NewEnumerator0"))
  (set `self.CurrentFaction` CurrentFaction))