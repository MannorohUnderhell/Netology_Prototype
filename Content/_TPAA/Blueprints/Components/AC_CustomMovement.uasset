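; AC_CustomMovement is an actor component that applies the owner's stat-driven walk speed when play begins.
; It reads MaxWalkSpeed from the owner's main stats struct, fetched through a message call rather than a cast.
; If the owner has a CharacterMovementComponent, it sets walk speed and half that for crouching, then calls CallOnCustomMovement.
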(event `self.ReceiveBeginPlay`
  (`self.ConfigureMovement`))

(fn `ConfigureMovement`
  (locals (L_MaxWalkSpeed :type "Float (double-precision)"))
  (bind _returnvalue (`Actor.GetComponentByClass` (`self.GetOwner`) "/Script/Engine.CharacterMovementComponent"))
  (bind (_success _mainstats) (message `/Game/_TPAA/Blueprints/GameEntities/BI_Stats.GetMainStatsStruct` (`self.GetOwner`)))
  (set `local.L_MaxWalkSpeed` (`.MaxWalkSpeed_11_255F0D4946058ED6A05A73AEB809F6C1` (break `/Game/_TPAA/Blueprints/Structures/STRUCT_MainStats` _mainstats)))
  (`/Engine/EditorBlueprintResources/StandardMacros.IsValid` _returnvalue
    (:`Is Valid`
      (set `CharacterMovementComponent.MaxWalkSpeed` (`local.L_MaxWalkSpeed`) _returnvalue)
      (set `CharacterMovementComponent.MaxWalkSpeedCrouched` (/ (`local.L_MaxWalkSpeed`) 2.0) _returnvalue)
      (`self.OnCustomMovement`))))