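; AC_HintWidget is a component that shows an interaction hint over its owning actor when a camera-bearing actor overlaps it.
; On BeginPlay it adds a screen-space WidgetComponent holding a WBP_Hint, snapped to its own transform, and binds the owner's overlap events.
; Overlaps store or clear the overlapping actor, set the ready-to-interact flag and animate the hint's visibility.
; Hint text falls back to a custom default when given empty text.
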(event `self.ReceiveBeginPlay`
  (`self.ConstructWidgetHint`)
  (add `Actor.OnActorBeginOverlap` (`self.GetOwner`) (`|CreateDelegate` :!event `OnActorBeginOverlap_Event`))
  (add `Actor.OnActorEndOverlap` (`self.GetOwner`) (`|CreateDelegate` :!event `OnActorEndOverlap_Event`)))

(event `OnActorBeginOverlap_Event`
  (params (OverlappedActor :type "Actor Object Reference") (OtherActor :type "Actor Object Reference"))
  (`/Engine/EditorBlueprintResources/StandardMacros.IsValid` (`Actor.GetComponentByClass` OtherActor "/Script/Engine.CameraComponent")
    (:`Is Valid`
      (set `self.ActorOnOverlap` OtherActor)
      (`self.UpdateHintVisibility` true)
      (set `self.bIsReadyToInteract` true))))

(event `OnActorEndOverlap_Event`
  (params (OverlappedActor :type "Actor Object Reference") (OtherActor :type "Actor Object Reference"))
  (`/Engine/EditorBlueprintResources/StandardMacros.IsValid` (`Actor.GetComponentByClass` OtherActor "/Script/Engine.CameraComponent")
    (:`Is Valid`
      (set `self.ActorOnOverlap` null)
      (`self.UpdateHintVisibility` false)
      (set `self.bIsReadyToInteract` false))))

(fn `ConstructWidgetHint`
  (`|ExecutionSequence`
    (:`then_0`
      (`self.WidgetComponent`
        (:`then`)
        (:`else`
          (bind _returnvalue (`|AddComponentByClass` (`self.GetOwner`) "/Script/UMG.WidgetComponent" false (`self.GetRelativeTransform`)))
          (set `self.WidgetComponent` _returnvalue))))
    (:`then_1`
      (`self.WidgetComponent`
        (:`then`
          (bind _returnvalue_2 (`|CreateWidget` "/Game/_TPAA/UI/Widgets/WBP_Hint.WBP_Hint_C" (`GameplayStatics.GetPlayerController` 0)))
          (set `self.HintWidget` _returnvalue_2)
          (`WidgetComponent.SetWidget` (`self.WidgetComponent`) (`self.HintWidget`))
          (`WidgetComponent.SetWidgetSpace` (`self.WidgetComponent`) "Screen")
          (`self.K2_AttachToComponent` (`self.WidgetComponent`) self "None" "SnapToTarget" "SnapToTarget" "KeepRelative" true))
        (:`else`)))
    (:`then_2`
      (`self.UpdateHintText` ""))))

(fn `UpdateHintText`
  (params (InText :type Text))
  (`self.HintWidget`
    (:`then`
      (set `TextBlock.Text` (`KismetMathLibrary.SelectText` (`self.CustomHintText`) (`local.InText`) (`KismetTextLibrary.TextIsEmpty` (`local.InText`))) (`/Game/_TPAA/UI/Widgets/WBP_Hint.HintText` (`self.HintWidget`))))
    (:`else`)))

(fn `UpdateHintVisibility`
  (params (bInIsItVisible :type Boolean :default true))
  (`/Game/_TPAA/UI/Widgets/WBP_Hint.PlayVisibilityAnimation` (`self.HintWidget`) (`local.bInIsItVisible`)))