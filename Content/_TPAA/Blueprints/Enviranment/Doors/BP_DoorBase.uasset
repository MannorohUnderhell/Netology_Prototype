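; Base interactable hinged door that swings open or closed when an actor calls Interact.
; A dot product between its Arrow and the interacting actor picks the swing direction, which is remembered so closing retraces the same arc.
; A timeline scales DoorScene yaw up to the max angle, with mesh collision and re-triggering disabled while it moves.
; The construction script previews the initial open state and sizes the box collision.
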(event `self.ReceiveBeginPlay`
  (`TimelineComponent.SetPlayRate` (`self.DoorProgressTimeline`) (`self.DoorOpenSpeed`)))

(event `OpenDoor`
  (if (not (`self.bInProgress`))
    (if (not (`self.bIsDoorOpen`))
      (`self.UpdateInProgress` true)
      (bind (_direction _dooropenprogress) (`Timeline|DoorProgressTimeline` :!via `PlayFromStart` :!label _label)
        (:`Update`
          (`SceneComponent.K2_SetRelativeRotation` (`self.DoorScene`) (`KismetMathLibrary.MakeRotator` 0.0 0.0 (* (`self.MaxDoorOpenAngle`) _dooropenprogress (`KismetMathLibrary.SelectFloat` (`self.PreviousDotProduct`) (`self.CurrentDotProduct`) (`self.bIsDoorOpen`)))) false false))
        (:`Finished`
          (set `self.PreviousDotProduct` (`self.CurrentDotProduct`))
          (`self.UpdateInProgress` false)
          (switch `ETimelineDirection` _direction
            (:`Forward`
              (set `self.bIsDoorOpen` true))
            (:`Backward`
              (set `self.bIsDoorOpen` false))))))))

(event `CloseDoor`
  (if (not (`self.bInProgress`))
    (if (`self.bIsDoorOpen`)
      (`self.UpdateInProgress` true)
      (goto _label :!via `ReverseFromEnd`))))

(fn `ConfigureOpenDoorOnConstruct`
  (`SceneComponent.K2_SetRelativeRotation` (`self.DoorScene`) (`KismetMathLibrary.MakeRotator` 0.0 0.0 (`KismetMathLibrary.SelectFloat` (`self.MaxDoorOpenAngle`) 0.0 (`self.bIsDoorOpen`))) false false))

(fn `Interact`
  (params (InteractActor :type "Actor Object Reference"))
  (returns (Success :type Boolean))
  (bind _output_get (set `self.ActorOfInteraction` InteractActor))
  (set `self.CurrentDotProduct` (`KismetMathLibrary.SelectFloat` 1.0 -1.0 (> (`/Game/_TPAA/Blueprints/GameEntities/BFL_TPAA.DotProductOfTwoComponents` (`self.Arrow`) (`Actor.RootComponent` _output_get)) 0.0)))
  (`self.UpdateDoorVisual`)
  (return true))

(fn `SwitchDoorOpen`
  (set `self.bIsDoorOpen` (not (`self.bIsDoorOpen`))))

(fn `UpdateBoxExtent`
  (bind (_doorboxcollisionextent_x _doorboxcollisionextent_y _doorboxcollisionextent_z) (`KismetMathLibrary.BreakVector` (`self.DoorBoxCollisionExtent`)))
  ; Locations update on construction
  (`BoxComponent.SetBoxExtent` (`self.DoorBoxCollision`) (`self.DoorBoxCollisionExtent`) true)
  (`SceneComponent.K2_SetRelativeLocation` (`self.DoorBoxCollision`) (`KismetMathLibrary.MakeVector` 0.0 0.0 _doorboxcollisionextent_z) false false))

(fn `UpdateDoorVisual`
  (if (`self.bIsDoorOpen`)
    (`self.CloseDoor`)
    (else
      (`self.OpenDoor`))))

(fn `UpdateInProgress`
  (params (bInProgress :type Boolean))
  (set `self.bInProgress` bInProgress)
  (`PrimitiveComponent.SetCollisionEnabled` (`self.DoorMesh`) (select `bool` (`self.bInProgress`) :`false` "QueryAndPhysics" :`true` "NoCollision" :!type "ECollisionEnabled Enum")))

(fn `UserConstructionScript`
  (`|ExecutionSequence`
    (:`then_0`
      (`self.ConfigureOpenDoorOnConstruct`))
    (:`then_1`
      (`self.UpdateBoxExtent`))))