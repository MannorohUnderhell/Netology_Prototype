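; BP_DoorWithLock is a child door Blueprint that adds a locked state with front and back lock icon meshes.
; While locked, the door starts closed, shows the icons, and a visual update plays a timeline that yaws the door slightly, scaled by a dot-product value, instead of running parent behavior.
; UnlockDoor clears the lock, swaps both icons to an open-lock mesh, then hides them after a short delay.
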(event `TryOpenLockedDoor`
  (bind (_direction _doorlockedtryingprogress) (`Timeline|LockedFeedbackTimeline` :!via `PlayFromStart`)
    (:`Update`
      (`SceneComponent.K2_SetRelativeRotation` (`self.DoorScene`) (`KismetMathLibrary.MakeRotator` 0.0 0.0 (* (`self.LockedDoorAngle`) _doorlockedtryingprogress (`self.CurrentDotProduct`))) false false))))

(event `UnlockFeedback`
  (`StaticMeshComponent.SetStaticMesh` (`self.LockClosedMeshF`) "/Game/Polygon_Prototype/Meshes/Icons/SM_Icon_Lock_Open_01.SM_Icon_Lock_Open_01")
  (`StaticMeshComponent.SetStaticMesh` (`self.LockClosedMeshB`) "/Game/Polygon_Prototype/Meshes/Icons/SM_Icon_Lock_Open_01.SM_Icon_Lock_Open_01")
  (`KismetSystemLibrary.Delay` 2.0)
  (`SceneComponent.SetVisibility` (`self.LockClosedMeshF`) false false)
  (`SceneComponent.SetVisibility` (`self.LockClosedMeshB`) false false))

(fn `ConfigureOpenDoorOnConstruct`
  (if (`self.bIsDoorLocked`)
    (set `self.bIsDoorOpen` (not (`self.bIsDoorLocked`))))
  (`parent.ConfigureOpenDoorOnConstruct`))

(fn `UnlockDoor`
  (set `self.bIsDoorLocked` false)
  (`self.UnlockFeedback`))

(fn `UpdateDoorVisual`
  (if (not (`self.bIsDoorLocked`))
    (`parent.UpdateDoorVisual`)
    (else
      (`self.TryOpenLockedDoor`))))

(fn `UserConstructionScript`
  (`parent.UserConstructionScript`)
  (`SceneComponent.SetVisibility` (`self.LockClosedMeshF`) (`self.bIsDoorLocked`) false)
  (`SceneComponent.SetVisibility` (`self.LockClosedMeshB`) (`self.bIsDoorLocked`) false))