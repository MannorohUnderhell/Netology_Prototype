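; BP_TooltipLookAt is an environment trigger that turns its Arrow component to face the camera of the overlapped actor, presumably to orient a tooltip.
; Each Tick it looks up a CameraComponent on OverlappedActor and, if both are valid, sets the Arrow's world rotation with FindLookAtRotation.
; The construction script only calls its parent, and the graphs shown never set OverlappedActor.
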(event `self.ReceiveTick`
  (params (DeltaSeconds :type "Float (single-precision)"))
  (`self.LookingAtPlayerCamera`))

(fn `LookingAtPlayerCamera`
  (bind _overlappedactor (`self.OverlappedActor`)
    (:`then`
      (bind _returnvalue (`self.GetComponentByClass` _overlappedactor "/Script/Engine.CameraComponent"))
      (`/Engine/EditorBlueprintResources/StandardMacros.IsValid` _returnvalue
        (:`Is Valid`
          (`SceneComponent.K2_SetWorldRotation` (`self.Arrow`) (`KismetMathLibrary.FindLookAtRotation` (`SceneComponent.K2_GetComponentLocation` (`self.Arrow`)) (`SceneComponent.K2_GetComponentLocation` _returnvalue)) false false))))
    (:`else`)))

(fn `UserConstructionScript`
  (`parent.UserConstructionScript`))