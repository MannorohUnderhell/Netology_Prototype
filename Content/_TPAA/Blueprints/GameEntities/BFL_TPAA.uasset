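; BFL_TPAA is a Blueprint function library of shared helpers for debug printing, facing math and stats lookup.
; PrintScreenCustom wraps PrintString with logging disabled, and DotProductOfTwoComponents compares one component's forward vector with the normalized direction to another.
; GetMainStatsStructByName reads a row from DT_AllStats by name; a missing row prints an error but still returns Success as true, without stats.
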(fn `DotProductOfTwoComponents`
  (params (InSceneComponentFromDotProduct :type "SceneComponent Object Reference") (InSceneComponentToDotProduct :type "SceneComponent Object Reference"))
  (returns (OutDotProductResult :type "Float (double-precision)"))
  (bind _inscenecomponentfromdotproduct (`local.InSceneComponentFromDotProduct`))
  (return (`KismetMathLibrary.Dot_VectorVector` (`KismetMathLibrary.Normal` (- (`SceneComponent.K2_GetComponentLocation` InSceneComponentToDotProduct) (`SceneComponent.K2_GetComponentLocation` _inscenecomponentfromdotproduct))) (`SceneComponent.GetForwardVector` _inscenecomponentfromdotproduct))))

(fn `GetMainStatsStructByName`
  (params (InName :type Name))
  (returns (Success :type Boolean) (MainStats :type "/Game/_TPAA/Blueprints/Structures/STRUCT_MainStats Structure"))
  (bind _returnvalue (`|GetDataTableRow` "/Game/_TPAA/Blueprints/DataTables/DT_AllStats.DT_AllStats" InName)
    (:`then`
      (return true _returnvalue))
    (:`RowNotFound`
      (`KismetSystemLibrary.PrintString` null "Configure Stats Failed: Current Name not found in DT" false)
      (return true))))

(fn `PrintScreenCustom`
  (params (InString :type String) (bPrintToScreen :type Boolean :default true) (TextColor :type "LinearColor Structure" :default (struct :`R` 1.0 :`A` 1.0)) (Duration :type "Float (single-precision)" :default 5.0) (Key :type Name))
  (`KismetSystemLibrary.PrintString` null InString bPrintToScreen false TextColor Duration Key))